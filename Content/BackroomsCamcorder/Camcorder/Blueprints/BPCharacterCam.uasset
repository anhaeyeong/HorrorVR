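; First-person character Blueprint that holds a camcorder with a scene-capture component, display, recording indicator and front light.
; Holding left mouse drives the arms AnimBlueprint's TakeUp and the recording state, while F toggles its HoldStart pose flag.
; R toggles the spotlight and its lens glow, and J cycles the battery bars.
; Helper functions push these states into material scalar parameters, and the character hides its own components from the capture.
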(event `self.ReceiveBeginPlay`
  (bind _assk_camcorder_anim_blueprint (cast `/Game/BackroomsCamcorder/Camcorder/Blueprints/SK_Camcorder_AnimBlueprint` (`SkeletalMeshComponent.GetAnimInstance` (`self.Equipment`))))
  (set `self.CamAnim` _assk_camcorder_anim_blueprint)
  (bind _assk_mannequin_arms_skeleton_anim_blueprint_cam (cast `/Game/BackroomsCamcorder/Camcorder/Blueprints/SK_Mannequin_Arms_Skeleton_AnimBlueprintCam` (`SkeletalMeshComponent.GetAnimInstance` (`self.SK_Mannequin_Arms`))))
  (set `self.ArmsAnim` _assk_mannequin_arms_skeleton_anim_blueprint_cam)
  ;[1 1 1] Hide ourself from the scene capture for the camcorder
  (`SceneCaptureComponent.HideActorComponents` (`self.SceneCaptureComponent2D`) self false)
  (`self.SetBatteryBars` 3)
  (`self.SetRecording` false))

(event `Key|LeftMouseButton`
  (params (Key :type "Key Structure"))
  (bind _armsanim (`self.ArmsAnim`))
  (:`Pressed`
    (set `/Game/BackroomsCamcorder/Camcorder/Blueprints/SK_Mannequin_Arms_Skeleton_AnimBlueprintCam.TakeUp` true _armsanim)
    (`self.SetRecording` (`/Game/BackroomsCamcorder/Camcorder/Blueprints/SK_Mannequin_Arms_Skeleton_AnimBlueprintCam.TakeUp` _armsanim) :!label _label))
  (:`Released`
    (set `/Game/BackroomsCamcorder/Camcorder/Blueprints/SK_Mannequin_Arms_Skeleton_AnimBlueprintCam.TakeUp` false _armsanim)
    (goto _label)))

(event `Key|F`
  (params (Key :type "Key Structure"))
  (:`Pressed`
    (bind _isa (`/Engine/EditorBlueprintResources/StandardMacros.FlipFlop`)
      (:`A`
        _)
      (:`B`
        _))
    (set `/Game/BackroomsCamcorder/Camcorder/Blueprints/SK_Mannequin_Arms_Skeleton_AnimBlueprintCam.HoldStart` _isa (`self.ArmsAnim`))))

(event `Key|R`
  (params (Key :type "Key Structure"))
  (:`Pressed`
    (bind _isa (`/Engine/EditorBlueprintResources/StandardMacros.FlipFlop`)
      (:`A`
        _)
      (:`B`
        _))
    (`self.SetFrontLight` _isa)))

(event `Key|J`
  (params (Key :type "Key Structure"))
  (:`Pressed`
    (`|MultiGate` false true 0
      (:`Out 0`
        (`self.SetBatteryBars` 1))
      (:`Out 1`
        (`self.SetBatteryBars` 2))
      (:`Out 2`
        (`self.SetBatteryBars` 3)))))

(fn `SetBatteryBars`
  (params (NumBarsToShow :type Integer))
  (bind _displayrt (`self.DisplayRT`))
  (`MeshComponent.SetScalarParameterValueOnMaterials` _displayrt "1bar" (`KismetMathLibrary.SelectFloat` 1.0 0.0 (== NumBarsToShow 1)))
  (`MeshComponent.SetScalarParameterValueOnMaterials` _displayrt "2bar" (`KismetMathLibrary.SelectFloat` 1.0 0.0 (== NumBarsToShow 2)))
  (`MeshComponent.SetScalarParameterValueOnMaterials` _displayrt "3bar" (`KismetMathLibrary.SelectFloat` 1.0 0.0 (== NumBarsToShow 3))))

(fn `SetFrontLight`
  (params (Enable :type Boolean))
  (`SceneComponent.SetVisibility` (`self.SpotLight`) Enable false)
  (`MeshComponent.SetScalarParameterValueOnMaterials` (`self.Equipment`) "FrontLight" (`KismetMathLibrary.SelectFloat` 100.0 0.0 Enable)))

(fn `SetRecording`
  (params (Recording :type Boolean))
  (bind _returnvalue (select `bool` Recording :`true` 1.0 :!type "Float (single-precision)"))
  (`MeshComponent.SetScalarParameterValueOnMaterials` (`self.DisplayRT`) "IsRecording" _returnvalue)
  (`MeshComponent.SetScalarParameterValueOnMaterials` (`self.Equipment`) "RecLightIntensity" (* _returnvalue 120.0)))

(fn `UserConstructionScript`)